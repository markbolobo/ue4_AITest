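; BP_Sekiro_GameController is the top-level update driver for the Sekiro game's character and AI manager.
; InitGameController stores both references and sets an initialized flag.
; Event Tick calls TickGameController, which, once initialized, manually ticks the character first and the AI manager second, giving a central, ordered update.
; SpecialMotionBoost is exposed as a parameter but is not forwarded; both calls receive zero.
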(event `self.ReceiveTick`
  (params (DeltaSeconds :type "Float (single-precision)"))
  (`self.TickGameController` DeltaSeconds))

(fn `InitGameController`
  (params (Character :type "/Game/Sekiro/Blueprints/BP_Sekiro_Character Object Reference") (AIManager :type "/Game/Sekiro/Blueprints/AISystem/Blueprints/BP_Sekiro_AICharacterManager Object Reference"))
  (set `self.mCharacter` Character)
  (set `self.mAIManager` AIManager)
  (set `self.mIsInitialize` true))

(fn `TickGameController`
  (params (DeltaSeconds :type "Float (double-precision)") (SpecialMotionBoost :type "Float (double-precision)"))
  (if (`self.mIsInitialize`)
    (`/Game/Sekiro/Blueprints/BP_Sekiro_Character.TickCharacter` (`self.mCharacter`) (`local.DeltaSeconds`) 0.0)
    (`/Game/Sekiro/Blueprints/AISystem/Blueprints/BP_Sekiro_AICharacterManager.TickAIManager` (`self.mAIManager`) (`local.DeltaSeconds`) 0.0)))

(fn `UserConstructionScript`)