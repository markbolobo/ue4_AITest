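; BP_Sekiro_UIManager creates and manages on-screen HUD widgets: a crosshair and per-enemy detection meters.
; InitUIManager adds the crosshair to the viewport, and TickUIManager then ticks every active meter.
; SetDetectionMeter finds the meter bound to an AI character, creating or showing it on add and removing it from viewport and array otherwise.
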(fn `GetDesiredRotation`
  (returns (Rotation :type "Rotator Structure"))
  (return))

(fn `InitUIManager`
  (bind _returnvalue (`|CreateWidget` "/Game/Sekiro/Blueprints/WB_Crosshair.WB_Crosshair_C"))
  (set `self.mUICrosshair` _returnvalue)
  (`UserWidget.AddToViewport` (`self.mUICrosshair`) 0)
  (set `self.mIsInitialize` true))

(fn `SetDetectionMeter`
  (params (IsAdd :type Boolean) (AICharacter :type "/Game/Sekiro/Blueprints/AISystem/Blueprints/BP_Sekiro_AICharacter Object Reference"))
  (returns (IsUIShow :type Boolean))
  (locals (aTempAICharacter :type "/Game/Sekiro/Blueprints/AISystem/Blueprints/BP_Sekiro_AICharacter Object Reference") (aTempUI :type "/Game/Sekiro/Blueprints/WB_DetectionMeter Object Reference") (aIsAICharacterExist :type Boolean))
  (set `local.aTempAICharacter` AICharacter)
  (for _array_element (`self.mUIDetectionMeter`)
    (if (== (`/Game/Sekiro/Blueprints/WB_DetectionMeter.mAICharacter` _array_element) (`local.aTempAICharacter`))
      (set `local.aTempUI` _array_element)
      (set `local.aIsAICharacterExist` true)
      (break)))
  (if (`local.aIsAICharacterExist`)
    (if IsAdd
      (`Widget.SetVisibility` (`local.aTempUI`) "Visible")
      (return true)
      (else
        (`Widget.RemoveFromParent` (`local.aTempUI`))
        (`KismetArrayLibrary.Array_RemoveItem` (`self.mUIDetectionMeter`) (`local.aTempUI`))
        (set `local.aTempUI` null)
        (return false)))
    (elif IsAdd
      (bind _returnvalue (`|CreateWidget` "/Game/Sekiro/Blueprints/WB_DetectionMeter.WB_DetectionMeter_C"))
      (set `local.aTempUI` _returnvalue)
      (`/Game/Sekiro/Blueprints/WB_DetectionMeter.InitUIDetectionMeter` (`local.aTempUI`) (`local.aTempAICharacter`))
      (`UserWidget.AddToViewport` (`local.aTempUI`) 0)
      (`KismetArrayLibrary.Array_AddUnique` (`self.mUIDetectionMeter`) (`local.aTempUI`))
      (return true))))

(fn `TickUIManager`
  (params (DeltaSeconds :type "Float (double-precision)") (SpecialMotionBoost :type "Float (double-precision)"))
  (if (`self.mIsInitialize`)
    (if (!= (`KismetArrayLibrary.Array_Length` (`self.mUIDetectionMeter`)) 0)
      (for _array_element (`self.mUIDetectionMeter`)
        (`/Game/Sekiro/Blueprints/WB_DetectionMeter.TickUIDetectionMeter` _array_element (`local.DeltaSeconds`))))))

(fn `UserConstructionScript`)