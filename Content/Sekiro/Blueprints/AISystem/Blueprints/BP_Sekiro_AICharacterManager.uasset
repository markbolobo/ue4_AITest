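; BP_Sekiro_AICharacterManager spawns, initializes and updates the enemy AI characters for the Sekiro game.
; InitAIManager spawns two character variants at hardcoded transforms, gives each a newly spawned possessing controller, then passes in the Character and UI manager.
; It tracks characters and controllers in arrays, caching the first of each separately.
; Once initialized, TickAIManager manually forwards delta time to every valid character, leaving its SpecialMotionBoost input unused.
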(fn `InitAIManager`
  (params (Character :type "/Game/Sekiro/Blueprints/BP_Sekiro_Character Object Reference") (UIManager :type "/Game/Sekiro/Blueprints/BP_Sekiro_UIManager Object Reference"))
  (`self.SpawnAICharacter`)
  (for _array_element (`self.mAllAICharacters`)
    (`/Game/Sekiro/Blueprints/AISystem/Blueprints/BP_Sekiro_AICharacter.InitAICharacter` _array_element Character UIManager))
  (set `self.mIsInitialize` true))

(fn `SpawnAICharacter`
  (bind _returnvalue (`|SpawnActorFromClass` "/Game/Sekiro/Blueprints/AISystem/Blueprints/BP_Sekiro_AICharacter.BP_Sekiro_AICharacter_C" (`KismetMathLibrary.MakeTransform` (-30.0 -180.0 418.0) (struct :`Yaw` 108.0)) "Undefined" "OverrideRootScale" null null))
  (`KismetArrayLibrary.Array_AddUnique` (`self.mAllAICharacters`) _returnvalue)
  (bind _returnvalue_2 (`|SpawnActorFromClass` "/Game/Sekiro/Blueprints/AISystem/Blueprints/BP_Sekiro_AICharacter_W.BP_Sekiro_AICharacter_W_C" (`KismetMathLibrary.MakeTransform` (-130.0 700.0 218.0) (struct :`Yaw` 108.0)) "Undefined" "OverrideRootScale" null null))
  (`KismetArrayLibrary.Array_AddUnique` (`self.mAllAICharacters`) _returnvalue_2)
  (for _array_element (`self.mAllAICharacters`)
    (bind _returnvalue_3 (`|SpawnActorFromClass` "/Game/Sekiro/Blueprints/BP_Sekiro_AIController.BP_Sekiro_AIController_C" (`KismetMathLibrary.MakeTransform` (0.0 0.0 0.0)) "Undefined" "OverrideRootScale" null null))
    (`KismetArrayLibrary.Array_AddUnique` (`self.mAllAIController`) _returnvalue_3)
    (`Controller.Possess` _returnvalue_3 _array_element))
  (set `self.AIController` (`|GetArrayItem` (`self.mAllAIController`)))
  (set `self.AICharacter` (`|GetArrayItem` (`self.mAllAICharacters`))))

(fn `TickAIManager`
  (params (DeltaSeconds :type "Float (double-precision)") (SpecialMotionBoost :type "Float (double-precision)"))
  (if (`self.mIsInitialize`)
    (for _array_element (`self.mAllAICharacters`)
      (`/Engine/EditorBlueprintResources/StandardMacros.IsValid` _array_element
        (:`Is Valid`
          (`/Game/Sekiro/Blueprints/AISystem/Blueprints/BP_Sekiro_AICharacter.TickAICharacter` _array_element DeltaSeconds))))))

(fn `UserConstructionScript`)