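; Player controller for the Sekiro game that forwards player input to a stored character reference, MCharacter.
; Movement and camera axes, the Jump, Dodge, Block and Target actions, and four directional keys each call a matching character function, with separate pressed and released calls for buttons.
; InitPlayerController stores that reference; its node setting MIsInitialize is unconnected and never runs.
; The controller holds no gameplay logic, leaving every response to the character.
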(event `InputAxis|Turn` :overrideparent false
  (params (AxisValue :type "Float (single-precision)"))
  (`/Game/Sekiro/Blueprints/BP_Sekiro_Character.Turn` (`self.mCharacter`) AxisValue))

(event `InputAxis|MoveForward` :overrideparent false
  (params (AxisValue :type "Float (single-precision)"))
  (`/Game/Sekiro/Blueprints/BP_Sekiro_Character.MoveForward` (`self.mCharacter`) AxisValue))

(event `InputAxis|LookUp` :overrideparent false
  (params (AxisValue :type "Float (single-precision)"))
  (`/Game/Sekiro/Blueprints/BP_Sekiro_Character.LookUp` (`self.mCharacter`) AxisValue))

(event `InputAction|Jump` :overrideparent false
  (params (Key :type "Key Structure"))
  (:`Pressed`
    (`/Game/Sekiro/Blueprints/BP_Sekiro_Character.JumpPressed` (`self.mCharacter`)))
  (:`Released`
    (`/Game/Sekiro/Blueprints/BP_Sekiro_Character.JumpReleased` (`self.mCharacter`))))

(event `InputAxis|MoveRight` :overrideparent false
  (params (AxisValue :type "Float (single-precision)"))
  (`/Game/Sekiro/Blueprints/BP_Sekiro_Character.MoveRight` (`self.mCharacter`) AxisValue))

(event `Key|F`
  (params (Key :type "Key Structure")))

(event `InputAction|Target`
  (params (Key :type "Key Structure"))
  (:`Pressed`
    (`/Game/Sekiro/Blueprints/BP_Sekiro_Character.TargetPressed` (`self.mCharacter`)))
  (:`Released`
    (`/Game/Sekiro/Blueprints/BP_Sekiro_Character.TargetReleased` (`self.mCharacter`))))

(event `InputAction|Dodge`
  (params (Key :type "Key Structure"))
  (:`Pressed`
    (`/Game/Sekiro/Blueprints/BP_Sekiro_Character.DodgePressed` (`self.mCharacter`)))
  (:`Released`
    (`/Game/Sekiro/Blueprints/BP_Sekiro_Character.DodgeReleased` (`self.mCharacter`))))

(event `Key|Left`
  (params (Key :type "Key Structure"))
  (:`Pressed`
    (`/Game/Sekiro/Blueprints/BP_Sekiro_Character.LeftPressed` (`self.mCharacter`)))
  (:`Released`
    (`/Game/Sekiro/Blueprints/BP_Sekiro_Character.LeftReleased` (`self.mCharacter`))))

(event `InputAction|Block`
  (params (Key :type "Key Structure"))
  (:`Pressed`
    (`/Game/Sekiro/Blueprints/BP_Sekiro_Character.BlockPressed` (`self.mCharacter`)))
  (:`Released`
    (`/Game/Sekiro/Blueprints/BP_Sekiro_Character.BlockReleased` (`self.mCharacter`))))

(event `Key|Right`
  (params (Key :type "Key Structure"))
  (:`Pressed`
    (`/Game/Sekiro/Blueprints/BP_Sekiro_Character.RightPressed` (`self.mCharacter`)))
  (:`Released`
    (`/Game/Sekiro/Blueprints/BP_Sekiro_Character.RightReleased` (`self.mCharacter`))))

(event `Key|Up`
  (params (Key :type "Key Structure"))
  (:`Pressed`
    (`/Game/Sekiro/Blueprints/BP_Sekiro_Character.UpPressed` (`self.mCharacter`)))
  (:`Released`
    (`/Game/Sekiro/Blueprints/BP_Sekiro_Character.UpReleased` (`self.mCharacter`))))

(event `Key|Down`
  (params (Key :type "Key Structure"))
  (:`Pressed`
    (`/Game/Sekiro/Blueprints/BP_Sekiro_Character.DownPressed` (`self.mCharacter`)))
  (:`Released`
    (`/Game/Sekiro/Blueprints/BP_Sekiro_Character.DownReleased` (`self.mCharacter`))))

(fn `InitPlayerController`
  (params (mCharacter :type "/Game/Sekiro/Blueprints/BP_Sekiro_Character Object Reference"))
  (set `self.mCharacter` mCharacter))

(fn `UserConstructionScript`)