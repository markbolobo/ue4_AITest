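; BP_Rotating is a roll-system component that turns its owner toward a desired rotation at a capped speed for a limited time.
; The window is given directly or derived from a maximum angle, though only the time-based start resets elapsed time.
; TickRotating uses constant interpolation toward the rotation the owner supplies by interface message.
; Expiry only halts turning; StopRotating clears the flag and fires the end callback.
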(fn `InitRotating`
  (set `self.mOwner` (`self.GetOwner`))
  (set `self.mIsInitialize` true))

(fn `IsRotating`
  (returns (IsShouldRotate :type Boolean))
  (return (`self.mIsShouldRotate`)))

(fn `StartRotatingWithLimit`
  (params (MaxPossibleRotation :type "Float (double-precision)" :default 180.0) (MaxDegreesPerSecond :type "Float (double-precision)" :default 720.0))
  (set `self.mRotateTime` (/ MaxPossibleRotation MaxDegreesPerSecond))
  (set `self.mMaxDegreesPerSecond` MaxDegreesPerSecond)
  (set `self.mIsShouldRotate` true)
  (`self.OnRotatingStart`))

(fn `StartRotatingWithTime`
  (params (Time :type "Float (double-precision)") (MaxDegreesPerSecond :type "Float (double-precision)" :default 720.0))
  (set `self.mRotateTime` Time)
  (set `self.mMaxDegreesPerSecond` MaxDegreesPerSecond)
  (set `self.mElapsedTick` 0.0)
  (set `self.mIsShouldRotate` true)
  (`self.OnRotatingStart`))

(fn `StopRotating`
  (set `self.mIsShouldRotate` false)
  (`self.OnRotatingEnd`))

(fn `TickRotating`
  (params (DeltaSeconds :type "Float (double-precision)"))
  (if (`self.mIsInitialize`)
    (if (`self.mIsShouldRotate`)
      (set `self.mElapsedTick` (+ (`self.mElapsedTick`) (`local.DeltaSeconds`)))
      (if (<= (`self.mElapsedTick`) (`self.mRotateTime`))
        (bind _rotation (message `/Game/Sekiro/Blueprints/BP_Sekiro_GameInterface.GetDesiredRotation` (`self.mOwner`)))
        (`Actor.K2_SetActorRotation` (`self.mOwner`) (`KismetMathLibrary.RInterpTo_Constant` (`Actor.K2_GetActorRotation` (`self.mOwner`)) _rotation (`local.DeltaSeconds`) (`self.mMaxDegreesPerSecond`)) false)))))