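; Bootstrap manager for the Sekiro game that creates and wires up the core gameplay objects on BeginPlay.
; It spawns the game controller, AI manager, player character and UI manager, and gets the existing player controller by casting player 0's controller.
; It then initializes each explicitly, passing the character to both controllers and the AI manager, and the AI manager to the game controller and character.
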(event `self.ReceiveBeginPlay`
  (`self.InitGameManager`))

(fn `InitGameManager`
  (bind _returnvalue (`|SpawnActorFromClass` "/Game/Sekiro/Blueprints/BP_Sekiro_GameController.BP_Sekiro_GameController_C" (`KismetMathLibrary.MakeTransform` (0.0 0.0 0.0)) "Undefined" "OverrideRootScale" null null))
  (set `self.mGameController` _returnvalue)
  (bind _returnvalue_2 (`|SpawnActorFromClass` "/Game/Sekiro/Blueprints/AISystem/Blueprints/BP_Sekiro_AICharacterManager.BP_Sekiro_AICharacterManager_C" (`KismetMathLibrary.MakeTransform` (0.0 0.0 0.0)) "Undefined" "OverrideRootScale" null null))
  (set `self.mAIManager` _returnvalue_2)
  (bind _returnvalue_3 (`|SpawnActorFromClass` "/Game/Sekiro/Blueprints/BP_Sekiro_Character.BP_Sekiro_Character_C" (`KismetMathLibrary.MakeTransform` (-750.0 400.0 226.284607)) "AlwaysSpawn" "OverrideRootScale" null null))
  (set `self.mCharacter` _returnvalue_3)
  (bind _asbp_sekiro_player_controller (cast `/Game/Sekiro/Blueprints/BP_Sekiro_PlayerController` (`GameplayStatics.GetPlayerController` 0)))
  (set `self.mPlayerController` _asbp_sekiro_player_controller)
  (bind _returnvalue_4 (`|SpawnActorFromClass` "/Game/Sekiro/Blueprints/BP_Sekiro_UIManager.BP_Sekiro_UIManager_C" (`KismetMathLibrary.MakeTransform` (-750.0 400.0 226.284607)) "AlwaysSpawn" "OverrideRootScale" null null))
  (set `self.mUIManager` _returnvalue_4)
  (`/Game/Sekiro/Blueprints/BP_Sekiro_GameController.InitGameController` (`self.mGameController`) (`self.mCharacter`) (`self.mAIManager`))
  (`/Game/Sekiro/Blueprints/AISystem/Blueprints/BP_Sekiro_AICharacterManager.InitAIManager` (`self.mAIManager`) (`self.mCharacter`))
  (`/Game/Sekiro/Blueprints/BP_Sekiro_PlayerController.InitPlayerController` (`self.mPlayerController`) (`self.mCharacter`))
  (`/Game/Sekiro/Blueprints/BP_Sekiro_Character.InitCharacter` (`self.mCharacter`) (`self.mAIManager`))
  (`/Game/Sekiro/Blueprints/BP_Sekiro_UIManager.InitUIManager` (`self.mUIManager`)))

(fn `UserConstructionScript`)