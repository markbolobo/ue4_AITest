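; BP_Sekiro_CharacterSpawnPoint is a numbered marker actor for a character spawn point in the Sekiro game.
; Until MIsInitialize is set, its construction script writes MIndex into a TextRender component and creates a dynamic instance of DefaultTextMaterialOpaque, passing the actor's yaw as a "Yaw" parameter.
; InitSpawnPoint only sets that flag, so later construction runs skip the label update.
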(fn `InitSpawnPoint`
  (set `self.mIsInitialize` true))

(fn `UserConstructionScript`
  (bind (_returnvalue_roll _returnvalue_pitch _returnvalue_yaw) (`KismetMathLibrary.BreakRotator` (`self.K2_GetActorRotation`)))
  (if (not (`self.mIsInitialize`))
    (`TextRenderComponent.K2_SetText` (`self.TextRender`) (`KismetTextLibrary.Conv_IntToText` (`self.mIndex`)))
    (bind _returnvalue (`PrimitiveComponent.CreateDynamicMaterialInstance` (`self.TextRender`) 0 "/Engine/EngineMaterials/DefaultTextMaterialOpaque.DefaultTextMaterialOpaque" "None"))
    (`MaterialInstanceDynamic.SetScalarParameterValue` _returnvalue "Yaw" _returnvalue_yaw)))