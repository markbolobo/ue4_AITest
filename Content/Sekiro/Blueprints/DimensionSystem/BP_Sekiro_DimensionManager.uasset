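; Manager Blueprint that tracks which numbered dimension each player occupies.
; SetPlayerDimension finds the player's entry in an array of player/dimension structs, offsets its dimension by a relative amount and clamps it to the configured range.
; It writes the entry back and prints debug messages for out-of-range requests and the resulting dimension.
; Init only sets an initialized flag, and the custom tick function checks it but does nothing yet.
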(fn `InitDimensionManager`
  (set `self.mIsInitialize` true))

(fn `SetPlayerDimension`
  (params (Player :type "/Game/Sekiro/Blueprints/BP_Sekiro_CharacterBase Object Reference (by ref)") (DimensionDifference :type "Integer (by ref)"))
  (locals (aTempNowDimension :type Integer) (aTempSetDimensionDifference :type Integer) (aTempSetPlayer :type "/Game/Sekiro/Blueprints/BP_Sekiro_CharacterBase Object Reference") (aTempPlayer :type "/Game/Sekiro/Blueprints/BP_Sekiro_CharacterBase Object Reference") (aTempInfo :type "/Game/Sekiro/Blueprints/DimensionSystem/S_Sekiro_DimensionInfo Structure") (aTempNewDimension :type Integer :default 0) (aTempMinDimension :type Integer :default 0) (aTempMaxDimension :type Integer :default 0) (aTempIndex :type Integer))
  (bind (_x _y) (`KismetMathLibrary.BreakVector2D` (`self.mDimensionRenge`)))
  (set `local.aTempSetPlayer` Player)
  (set `local.aTempSetDimensionDifference` DimensionDifference)
  (for (_array_element _array_index) (`self.mAllDimensionPlayers`)
    (set `local.aTempInfo` _array_element)
    (set `local.aTempIndex` _array_index)
    (set `local.aTempPlayer` (`.Player_2_98881D6C470CD7FCA0752DBAB7C8E1D3` (break `/Game/Sekiro/Blueprints/DimensionSystem/S_Sekiro_DimensionInfo` (`local.aTempInfo`))))
    (if (== (`local.aTempPlayer`) (`local.aTempSetPlayer`))
      (break)))
  (set `local.aTempNowDimension` (`.Dimension_5_9AB30DE441265B39AD056BB268D4359D` (break `/Game/Sekiro/Blueprints/DimensionSystem/S_Sekiro_DimensionInfo` (`local.aTempInfo`))))
  (set `local.aTempNewDimension` (+ (`local.aTempNowDimension`) (`local.aTempSetDimensionDifference`)))
  (`|ExecutionSequence`
    (:`then_0`
      (set `local.aTempMinDimension` (`KismetMathLibrary.FTrunc` _x))
      (set `local.aTempMaxDimension` (`KismetMathLibrary.FTrunc` _y)))
    (:`then_1`
      (if (> (`local.aTempNewDimension`) (`local.aTempMaxDimension`))
        (`KismetSystemLibrary.PrintString` "Over Max Dimension")
        (set `local.aTempNewDimension` (`KismetMathLibrary.Clamp` (`local.aTempNewDimension`) (`local.aTempMinDimension`) (`local.aTempMaxDimension`)) :!label _label)
        (elif (< (`local.aTempNewDimension`) (`local.aTempMinDimension`))
          (`KismetSystemLibrary.PrintString` "Lower Min Dimension")
          (goto _label))))
    (:`then_2`
      (`KismetArrayLibrary.Array_Set` (`self.mAllDimensionPlayers`) (`local.aTempIndex`) (make `/Game/Sekiro/Blueprints/DimensionSystem/S_Sekiro_DimensionInfo` (`local.aTempPlayer`) (`local.aTempNewDimension`)))
      (`KismetSystemLibrary.PrintString` (`KismetStringLibrary.Concat_StrStr` (`KismetSystemLibrary.GetDisplayName` (`local.aTempPlayer`)) " Now At Dimension " (`KismetStringLibrary.Conv_IntToString` (`local.aTempNewDimension`)))))))

(fn `TickDimensionManager`
  (params (DeltaSeconds :type "Float (double-precision)"))
  (if (`self.mIsInitialize`)
    _))

(fn `UserConstructionScript`)